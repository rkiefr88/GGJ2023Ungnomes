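; BP_Health tracks health for the player character and signals when it runs out.
; On BeginPlay it fills current health to maximum, casts player pawn 0 to BP_PlayerCharacter and binds to that character's OnTakeAnyDamage.
; Each hit subtracts damage, clamped between zero and maximum, and calls the OnDeath dispatcher whenever health is at zero.
; The damage source is always the first player pawn, regardless of where the Blueprint is placed.
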(event Custom|On%20Take%20Any%20Damage
  (params (DamagedActor :type Actor%20Object%20Reference) (Damage :type Float%20%28single-precision%29) (DamageType :type Damage%20Type%20Object%20Reference) (InstigatedBy :type Controller%20Object%20Reference) (DamageCauser :type Actor%20Object%20Reference))
  (Variables|Default|SetCurrent%20Health (Math|Float|Clamp(Float) (- (Variables|Default|GetCurrent%20Health) Damage) 0.0 (Variables|Default|GetMax%20Health)))
  (if (<= (Variables|Default|GetCurrent%20Health) 0.0)
    (Default|CallOnDeath)))

(event EventBeginPlay
  (Variables|Default|SetCurrent%20Health (Variables|Default|GetMax%20Health))
  (bind _asbp_player_character (Utilities|Casting|CastToBP_PlayerCharacter (Game|Player|GetPlayerPawn 0)))
  (bind _output_get (Variables|Default|SetAs%20BP%20Player%20Character _asbp_player_character))
  (EventDispatchers|BindEventtoOnTakeAnyDamage _output_get (delegate Custom|On%20Take%20Any%20Damage)))
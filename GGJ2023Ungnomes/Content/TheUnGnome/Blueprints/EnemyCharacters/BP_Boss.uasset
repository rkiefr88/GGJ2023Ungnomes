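; Boss enemy that alternates chasing the player with a pillar charge, and shows the win screen when killed.
; A latent AIMoveTo loop from BeginPlay chases the player's tracked location until four successful moves, then plays a stomp and speeds to the pillar nearest the player.
; Arrival triggers a timed, damageable stun before the chase resets.
; Box overlaps deal damage and re-enable chasing; a player hit ends vulnerability.
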(event OnComponentBeginOverlap(Box)
  (params (OverlappedComponent :type Primitive%20Component%20Object%20Reference) (OtherActor :type Actor%20Object%20Reference) (OtherComp :type Primitive%20Component%20Object%20Reference) (OtherBodyIndex :type Integer) (bFromSweep :type Boolean) (SweepResult :type Hit%20Result%20Structure%20%28by%20ref%29))
  ;[0.3542 0.3542 0.3542] Boss Damage Dealt
  (Game|Damage|ApplyDamage OtherActor 1.0 0 0)
  (Variables|Default|SetChase%20sequence true))

(event EventBeginPlay
  (bind _self self)
  ;[0.3059 1 0.2732] Begin Play // sets cureent health to max and set the player char var
  (Variables|Default|SetCurrent%20health (Variables|Default|GetMax%20Health))
  (bind _asbp_player_character (Utilities|Casting|CastToBP_PlayerCharacter (Game|Player|GetPlayerPawn 0)))
  (Variables|Default|SetAs%20BP%20Player%20Character _asbp_player_character)
  ;[1 0.8931 0] Chase Player
  (Utilities|FlowControl|Delay 4.0)
  (if (Variables|Default|GetChase%20sequence) :!label _label
    _
    (else
      ;[0.8325 0.1797 1] Stomp sequence
      (Rendering|SetVisibility (Variables|Default|GetParticleSystem1) true false)
      (Audio|PlaySoundatLocation "/Game/Magic___Spell_Sounds_PRO/General/wav/Buff_Attack_4.Buff_Attack_4" (Transformation|GetWorldLocation (Variables|Default|GetCube)) "0, 0, 0" 1.0 1.0 0.0 0 0 0)
      (Utilities|FlowControl|Delay 1.0)
      (Rendering|SetVisibility (Variables|Default|GetParticleSystem1) false false)
      (Variables|/Script/Engine.FloatingPawnMovement|SetMaxSpeed (Variables|Default|GetFloatingPawnMovement) 6e+02)
      (CallFunction|GetPlayerLocation)
      (if (> (Transformation|GetDistanceTo (Variables|Default|GetAs%20BP%20Player%20Character) (Variables|Default|GetLeft%20pillar)) (Transformation|GetDistanceTo (Variables|Default|GetAs%20BP%20Player%20Character) (Variables|Default|GetRight%20Pillar)))
        (AI|AIMoveTo _self (Variables|Default|GetRight%20Pillar%20Loc) 0 1e+01 false
          (:OnSuccess
            _))
        (else
          (AI|AIMoveTo _self (Variables|Default|GetLeft%20Pillar%20Loc) 0 1e+01 false
            (:OnSuccess
              _))))
      ;[0 0.1746 1] Stun Sequence and reset
      (Rendering|SetVisibility (Variables|Default|GetParticleSystem) true false)
      (Variables|Actor|SetbCanBeDamaged true)
      (Utilities|FlowControl|Delay 4.0)
      (Variables|Default|SetChase%20sequence true)
      (Variables|Default|Setchase%20num 0.0)
      (Variables|Actor|SetbCanBeDamaged false)
      (Variables|/Script/Engine.FloatingPawnMovement|SetMaxSpeed (Variables|Default|GetFloatingPawnMovement) 3e+02)
      (Rendering|SetVisibility (Variables|Default|GetParticleSystem) false false)))
  (CallFunction|GetPlayerLocation :!label _label_2)
  (AI|AIMoveTo self (Variables|Default|GetAI%20Move%20To) 0 5.0 false
    (:OnSuccess
      (bind _result (Math|Float|IncrementFloat (Variables|Default|Getchase%20num))
        (:%20%20
          (Variables|Default|Setchase%20num _result)
          (CallFunction|GetPlayerLocation)
          (Utilities|FlowControl|Delay 1.0)
          (goto _label))))
    (:OnFail
      (goto _label_2))))

(event Game|Damage|EventAnyDamage
  (params (Damage :type Float%20%28single-precision%29) (DamageType :type Damage%20Type%20Object%20Reference) (InstigatedBy :type Controller%20Object%20Reference) (DamageCauser :type Actor%20Object%20Reference))
  ;[1 0.07812 0.07812] Boss Owch
  (Utilities|Casting|CastToBP_PlayerCharacter DamageCauser)
  (Variables|Default|SetCurrent%20health (- (Variables|Default|GetCurrent%20health) Damage))
  (Variables|Actor|SetbCanBeDamaged false)
  (Rendering|SetVisibility (Variables|Default|GetParticleSystem) false false)
  ;[0.4531 0.03923 0] Boss Death
  (if (<= (Math|Float|Clamp(Float) (Variables|Default|GetCurrent%20health) 0.0 (Variables|Default|GetMax%20Health)) 0.0)
    (Actor|DestroyActor)
    (bind _returnvalue (UserInterface|CreateWidget "/Game/TheUnGnome/GUI/WBP_WinScreen.WBP_WinScreen_C"))
    (bind _output_get (Variables|Default|SetW_Win _returnvalue))
    (UserInterface|Viewport|AddtoViewport _output_get 0)))

(event EventTick
  (params (DeltaSeconds :type Float%20%28single-precision%29))
  ;[0 0 0] Keeps track of player location for the AI
  (CallFunction|GetPlayerLocation)
  (if (== (Variables|Default|Getchase%20num) 4.0)
    (Variables|Default|SetChase%20sequence false)))

(fn ConstructionScript)

(fn GetPlayerLocation
  (bind _asbp_player_character (Utilities|Casting|CastToBP_PlayerCharacter (Game|Player|GetPlayerPawn 0)))
  (Variables|Default|SetAI%20Move%20To (Transformation|GetWorldLocation (Variables|/Script/Engine.Character|GetMesh _asbp_player_character)))
  (return))
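; BP_Mushroom is a bouncy mushroom pad that launches the player character when it enters the Box trigger.
; The overlap restarts the MushroomBounce timeline, which wiggles the head and stem scales and moves the head along Z.
; A DoOnce on the timeline update plays a pop sound and launches the player along the Arrow's forward vector by LaunchForce, overriding current velocity.
; The DoOnce resets when the timeline finishes or the player leaves the box.
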(event OnComponentBeginOverlap(Box)
  (params (OverlappedComponent :type Primitive%20Component%20Object%20Reference) (OtherActor :type Actor%20Object%20Reference) (OtherComp :type Primitive%20Component%20Object%20Reference) (OtherBodyIndex :type Integer) (bFromSweep :type Boolean) (SweepResult :type Hit%20Result%20Structure%20%28by%20ref%29))
  (bind _headse (Variables|Default|GetHeadSE))
  (bind _asbp_player_character (Utilities|Casting|CastToBP_PlayerCharacter OtherActor))
  (bind (_direction _headwiggle _stimwiggle _movehead) (Timeline|MushroomBounce PlayFromStart)
    (:Update
      (Transformation|SetRelativeScale3D _headse (Math|Conversions|ToVector(Float) _headwiggle))
      (Transformation|SetRelativeScale3D (Variables|Default|GetSTemSE) (Math|Vector|MakeVector _stimwiggle 1.0 _stimwiggle))
      (Transformation|SetRelativeLocation _headse (Math|Vector|MakeVector 0.0 0.0 _movehead) false false)
      (Utilities|FlowControl|DoOnce false :!label _label
        (:Completed
          (Audio|PlaySoundatLocation "/Game/InterfaceAndItemSounds/Cues/Pop_04_wav_Cue.Pop_04_wav_Cue" (Transformation|GetWorldLocation (Variables|Default|GetSphere)) "0, 0, 0" 1.0 1.0 0.0 0 0 0)
          (Character|LaunchCharacter _asbp_player_character (* (Math|Vector|GetForwardVector (Variables|Default|GetArrow)) (Variables|Default|GetLaunchForce)) true true))))
    (:Finished
      (goto _label Reset))))

(event OnComponentEndOverlap(Box)
  (params (OverlappedComponent :type Primitive%20Component%20Object%20Reference) (OtherActor :type Actor%20Object%20Reference) (OtherComp :type Primitive%20Component%20Object%20Reference) (OtherBodyIndex :type Integer))
  (Utilities|Casting|CastToBP_PlayerCharacter OtherActor)
  (Utilities|FlowControl|DoOnce false) ; enters at Reset
)

(event EventBeginPlay)

(event EventTick
  (params (DeltaSeconds :type Float%20%28single-precision%29)))

(fn ConstructionScript)
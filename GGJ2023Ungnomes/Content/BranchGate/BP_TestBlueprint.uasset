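; Interactable root actor in the BranchGate folder that wiggles and retracts, then destroys itself.
; Interact sets the RetractRoot timeline's play rate from the mesh's current Z scale, triggers HealingRoot and returns false.
; HealingRoot plays the timeline, whose Wiggling and Retract tracks drive the mesh's pitch and Z scale until the actor is destroyed on finish.
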(event Custom|HealingRoot
  (bind _staticmesh (Variables|Default|GetStaticMesh))
  (bind _returnvalue (Transformation|GetRelativeTransform _staticmesh))
  (bind _relativerotation (Variables|/Script/Engine.SceneComponent|GetRelativeRotation _staticmesh))
  (bind (_direction _retract _wiggling) (Timeline|retractRoot Play)
    (:Update
      (Transformation|SetRelativeRotation _staticmesh (Math|Rotator|MakeRotator (.roll _relativerotation) _wiggling (.yaw _relativerotation)) false false)
      (Transformation|SetRelativeScale3D _staticmesh (Math|Vector|MakeVector (.x (.scale _returnvalue)) (.y (.scale _returnvalue)) _retract)))
    (:Finished
      (Actor|DestroyActor))))

(fn ConstructionScript)

(fn Interact
  (params (Interacter :type Character%20Object%20Reference))
  (Components|Timeline|SetPlayRate (Variables|Default|GetretractRoot) (/ (.z (.scale (Transformation|GetRelativeTransform (Variables|Default|GetStaticMesh)))) 1.0))
  (CallFunction|HealingRoot)
  (return false))
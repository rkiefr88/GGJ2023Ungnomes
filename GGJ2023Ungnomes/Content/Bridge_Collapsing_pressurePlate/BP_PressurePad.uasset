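; Pressure pad that triggers a collapsing bridge when something overlaps its box trigger.
; The overlap destroys the referenced Target actor and enables physics simulation on Woodplank1 and Woodplank6 so they move freely.
; The validity check on Target gates the whole response, so nothing happens once that actor is gone.
; A timeline that would lerp both planks' rotations between start and end positions is present but never runs.
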(event OnComponentBeginOverlap(Box)
  (params (OverlappedComponent :type Primitive%20Component%20Object%20Reference) (OtherActor :type Actor%20Object%20Reference) (OtherComp :type Primitive%20Component%20Object%20Reference) (OtherBodyIndex :type Integer) (bFromSweep :type Boolean) (SweepResult :type Hit%20Result%20Structure%20%28by%20ref%29))
  (bind _target (Variables|Default|GetTarget))
  (Utilities|IsValid _target
    (:Is%20Valid
      (Actor|DestroyActor _target)
      (for _array_element (Utilities|Array|MakeArray (Variables|Default|GetWoodplank1) (Variables|Default|GetWoodplank6))
        (Physics|SetSimulatePhysics _array_element true)))))

(fn ConstructionScript)